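; Sky sphere for a day/night cycle that drives a dynamic panning-cloud material with sun, moon and stars.
; The construction script sets it from optional sun and moon light actors, with colors from sun-height curves or manual values.
; UpdateSunDirection refreshes sun, curve colors and star blend, always using the curves.
; UpdateMoon sets moon direction, a slightly offset mask direction and elevation-switched brightness; BeginPlay is empty and calls neither.
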(event `self.ReceiveBeginPlay`)

(fn `UpdateMoon`
  (params (`Moon ELevation` :type "Float (double-precision)"))
  (bind _sky_material (`self.Sky material`))
  (bind _returnvalue (`self.K2_GetActorRotation` (`self.MoonLight Actor`)))
  (`MaterialInstanceDynamic.SetVectorParameterValue` _sky_material "MoonLight direction" (`KismetMathLibrary.Conv_VectorToLinearColor` (`KismetMathLibrary.Conv_RotatorToVector` _returnvalue)))
  (`MaterialInstanceDynamic.SetVectorParameterValue` _sky_material "MoonLightMask direction" (`KismetMathLibrary.Conv_VectorToLinearColor` (`KismetMathLibrary.Conv_RotatorToVector` (`KismetMathLibrary.MakeRotator` (.roll _returnvalue) (+ (.pitch _returnvalue) 1.0) (+ (.yaw _returnvalue) 1.0)))))
  (`MaterialInstanceDynamic.SetScalarParameterValue` (`self.Sky material`) "Moon brightness" (`KismetMathLibrary.SelectFloat` (`self.Moon Min brightness`) (`self.Moon brightness`) (> `Moon ELevation` -5.0))))

(fn `UpdateSunDirection`
  (bind _sky_material (`self.Sky material`))
  (bind _sun_height (`self.Sun height`))
  (bind _sun_height_2 (`self.Sun height`))
  (bind _sky_material_2 (`self.Sky material`))
  (`MaterialInstanceDynamic.SetVectorParameterValue` _sky_material "Light direction" (`KismetMathLibrary.Conv_VectorToLinearColor` (`KismetMathLibrary.Conv_RotatorToVector` (`self.K2_GetActorRotation` (`self.SunLight Actor`)))))
  (`MaterialInstanceDynamic.SetVectorParameterValue` _sky_material "Sun color" (`KismetMathLibrary.Conv_ColorToLinearColor` (`LightComponentBase.LightColor` (`Light.LightComponent` (`self.SunLight Actor`)))))
  (set `self.Sun height` (`KismetMathLibrary.MapRangeUnclamped` (.pitch (`self.K2_GetActorRotation` (`self.SunLight Actor`))) 0.0 -18.0 0.0 1.0))
  (`MaterialInstanceDynamic.SetVectorParameterValue` _sky_material_2 "Horizon color" (`CurveLinearColor.GetLinearColorValue` (`self.Horizon color curve`) (`self.Sun height`)))
  (`MaterialInstanceDynamic.SetVectorParameterValue` _sky_material_2 "Zenith color" (`CurveLinearColor.GetLinearColorValue` (`self.Zenith color curve`) (`self.Sun height`)))
  (`MaterialInstanceDynamic.SetVectorParameterValue` _sky_material_2 "Cloud color" (`CurveLinearColor.GetLinearColorValue` (`self.Cloud color curve`) _sun_height_2))
  (`MaterialInstanceDynamic.SetScalarParameterValue` _sky_material_2 "Horizon falloff" (`KismetMathLibrary.Lerp` 3.0 8.0 (`KismetMathLibrary.Abs` _sun_height_2)))
  (`MaterialInstanceDynamic.SetScalarParameterValue` _sky_material_2 "Sun height" (`KismetMathLibrary.SelectFloat` (`KismetMathLibrary.Abs` _sun_height) 0.0 (< _sun_height 0.0))))

(fn `UserConstructionScript`
  (bind _sky_material (`self.Sky material`))
  (bind _sky_material_2 (`self.Sky material`))
  (bind _sky_material_3 (`self.Sky material`))
  (bind _sun_height (`self.Sun height`))
  (bind _sun_height_2 (`self.Sun height`))
  (bind _sky_material_4 (`self.Sky material`))
  (bind _sky_material_5 (`self.Sky material`))
  (bind _returnvalue (`PrimitiveComponent.CreateDynamicMaterialInstance` (`self.Sky Sphere mesh`) 0 "/Game/Assets/DayNightCycle/Materials/M_Sky_Panning_Clouds2_Inst.M_Sky_Panning_Clouds2_Inst" "None"))
  (set `self.Sky material` _returnvalue)
  (if (`self.Refresh material`)
    _
    (else
      _))
  (set `self.Refresh material` false)
  (`/Engine/EditorBlueprintResources/StandardMacros.IsValid` (`self.SunLight Actor`) ; Has a directional light been assigned?
    (:`Is Valid`
      (`MaterialInstanceDynamic.SetVectorParameterValue` _sky_material_3 "Light direction" (`KismetMathLibrary.Conv_VectorToLinearColor` (`KismetMathLibrary.Conv_RotatorToVector` (`self.K2_GetActorRotation` (`self.SunLight Actor`)))))
      (`MaterialInstanceDynamic.SetVectorParameterValue` _sky_material_3 "Sun color" (`KismetMathLibrary.Conv_ColorToLinearColor` (`LightComponentBase.LightColor` (`Light.LightComponent` (`self.SunLight Actor`)))))
      (set `self.Sun height` (`KismetMathLibrary.MapRangeUnclamped` (.pitch (`self.K2_GetActorRotation` (`self.SunLight Actor`))) 10.0 0.0 0.0 1.0)))
    (:`Is Not Valid`
      (`MaterialInstanceDynamic.SetVectorParameterValue` _sky_material_2 "Light direction" (`KismetMathLibrary.Conv_VectorToLinearColor` (`KismetMathLibrary.Conv_RotatorToVector` (`KismetMathLibrary.MakeRotator` 0.0 (`KismetMathLibrary.MapRangeUnclamped` (`self.Sun height`) -1.0 1.0 90.0 -90.0) (.yaw (`self.K2_GetActorRotation`))))))
      (`MaterialInstanceDynamic.SetVectorParameterValue` _sky_material_2 "Sun color" (`KismetMathLibrary.LinearColorLerp` (struct :`R` 1.0 :`G` 0.221 :`B` 0.04 :`A` 1.0) (struct :`R` 0.954 :`G` 0.901 :`B` 0.74412 :`A` 1.0) (`KismetMathLibrary.FClamp` (+ (`self.Sun height`) 0.2))))))
  (`/Engine/EditorBlueprintResources/StandardMacros.IsValid` (`self.MoonLight Actor`)
    (:`Is Valid`
      (`MaterialInstanceDynamic.SetVectorParameterValue` (`self.Sky material`) "MoonLight direction" (`KismetMathLibrary.Conv_VectorToLinearColor` (`KismetMathLibrary.Conv_RotatorToVector` (`self.K2_GetActorRotation` (`self.MoonLight Actor`))))))
    (:`Is Not Valid`
      _))
  (if (`self.Colors determined by sun position`)
    (`MaterialInstanceDynamic.SetVectorParameterValue` _sky_material_4 "Horizon color" (`CurveLinearColor.GetLinearColorValue` (`self.Horizon color curve`) (`self.Sun height`)))
    (`MaterialInstanceDynamic.SetVectorParameterValue` _sky_material_4 "Zenith color" (`CurveLinearColor.GetLinearColorValue` (`self.Zenith color curve`) (`self.Sun height`)))
    (`MaterialInstanceDynamic.SetVectorParameterValue` _sky_material_4 "Cloud color" (`CurveLinearColor.GetLinearColorValue` (`self.Cloud color curve`) _sun_height_2))
    (`MaterialInstanceDynamic.SetScalarParameterValue` _sky_material_4 "Horizon falloff" (`KismetMathLibrary.Lerp` 3.0 7.0 (`KismetMathLibrary.Abs` _sun_height_2)))
    (else
      (`MaterialInstanceDynamic.SetVectorParameterValue` _sky_material "Horizon color" (`self.Horizon color`))
      (`MaterialInstanceDynamic.SetVectorParameterValue` _sky_material "Zenith color" (`self.Zenith Color`))
      (`MaterialInstanceDynamic.SetVectorParameterValue` _sky_material "Overall color" (`self.Overall Color`))
      (`MaterialInstanceDynamic.SetVectorParameterValue` _sky_material "Cloud color" (`self.Cloud color`))
      (`MaterialInstanceDynamic.SetScalarParameterValue` _sky_material "Horizon falloff" (`self.Horizon Falloff`))))
  (`MaterialInstanceDynamic.SetScalarParameterValue` _sky_material_5 "Cloud speed" (`self.Cloud speed`))
  (`MaterialInstanceDynamic.SetScalarParameterValue` _sky_material_5 "Sun brightness" (`self.Sun brightness`))
  (`MaterialInstanceDynamic.SetScalarParameterValue` _sky_material_5 "Sun height" (`KismetMathLibrary.SelectFloat` (`KismetMathLibrary.Abs` _sun_height) 0.0 (< _sun_height 0.0)))
  (`MaterialInstanceDynamic.SetScalarParameterValue` _sky_material_5 "Cloud opacity" (`self.Cloud opacity`))
  (`MaterialInstanceDynamic.SetScalarParameterValue` _sky_material_5 "Stars brightness" (`self.Stars brightness`)))